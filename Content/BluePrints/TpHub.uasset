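; TpHub is a hub teleport trigger that approves travel when the player is in range and carrying an object.
; Box overlap events track InRange and latch a Finish flag on first entry.
; TriggerTpHub checks HaveObj on the Player2D or MyCharacter pawn, copies its CurrentObject into MyGameInstance and returns true.
; TriggerTp returns no level and no teleport, so the level change is not performed here.
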(event `self.ReceiveBeginPlay`
  (set `self.finish` false))

(event `self.Box.OnComponentBeginOverlap`
  (params (OverlappedComponent :type "PrimitiveComponent Object Reference") (OtherActor :type "Actor Object Reference") (OtherComp :type "PrimitiveComponent Object Reference") (OtherBodyIndex :type Integer) (bFromSweep :type Boolean) (SweepResult :type "HitResult Structure (by ref)"))
  (set `self.inRange` true)
  (set `self.finish` true))

(event `self.Box.OnComponentEndOverlap`
  (params (OverlappedComponent :type "PrimitiveComponent Object Reference") (OtherActor :type "Actor Object Reference") (OtherComp :type "PrimitiveComponent Object Reference") (OtherBodyIndex :type Integer))
  (set `self.inRange` false))

(fn `TriggerTp`
  (returns (LevelName :type Name) (Teleport :type Boolean))
  (return "None" false))

(fn `TriggerTpHub`
  (returns (Teleport :type Boolean))
  (bind _returnvalue (`GameplayStatics.GetPlayerPawn` 0))
  (bind _asmy_game_instance (cast `/Game/MyGameInstance` (`GameplayStatics.GetGameInstance`)))
  (if (`self.inRange`)
    (bind _asplayer_2d (cast `/Game/Player2D` _returnvalue)
      (:`then`
        (if (`/Game/Player2D.HaveObj` _asplayer_2d)
          (set `/Game/MyGameInstance.currentObject` (`/Game/Player2D.CurrentObject` _asplayer_2d) _asmy_game_instance)
          (else
            (return false))))
      (:`CastFailed`
        (bind _asmy_character (cast `/Game/MyCharacter` _returnvalue))
        (if (`/Game/MyCharacter.HaveObj` _asmy_character)
          (set `/Game/MyGameInstance.currentObject` (`/Game/MyCharacter.CurrentObject` _asmy_character) _asmy_game_instance)
          (else
            (return false)))))
    (return true)
    (else
      (return false))))

(fn `UserConstructionScript`)