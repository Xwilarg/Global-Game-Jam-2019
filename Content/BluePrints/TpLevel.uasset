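; Level teleport trigger, apparently a computer, that decides whether the player can travel to its target level and returns the level name to the caller.
; A Box overlap tracks range; TriggerTp refuses when out of range, finished or the player carries an object, setting thought text for the latter two.
; On success it saves "Drop"-tagged actors' classes and transforms, plus the player transform, into MyGameInstance.
; TriggerTpHub always returns false.
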(event `self.ReceiveBeginPlay`
  (set `self.finish` false))

(event `self.Box.OnComponentBeginOverlap`
  (params (OverlappedComponent :type "PrimitiveComponent Object Reference") (OtherActor :type "Actor Object Reference") (OtherComp :type "PrimitiveComponent Object Reference") (OtherBodyIndex :type Integer) (bFromSweep :type Boolean) (SweepResult :type "HitResult Structure (by ref)"))
  (set `self.inRange` true))

(event `self.Box.OnComponentEndOverlap`
  (params (OverlappedComponent :type "PrimitiveComponent Object Reference") (OtherActor :type "Actor Object Reference") (OtherComp :type "PrimitiveComponent Object Reference") (OtherBodyIndex :type Integer))
  (set `self.inRange` false))

(fn `TriggerTp`
  (returns (LevelName :type Name) (Teleport :type Boolean))
  (bind _returnvalue (`GameplayStatics.GetPlayerPawn` 0))
  (if (`self.finish`)
    (bind _asmy_character (cast `/Game/MyCharacter` _returnvalue))
    (set `/Game/MyCharacter.ThinkContent` "It looks like the computer is off... " _asmy_character)
    (return "None" false)
    (else
      (bind _asmy_game_instance (cast `/Game/MyGameInstance` (`GameplayStatics.GetGameInstance`)))
      (if (`self.inRange`)
        (bind _asmy_character_2 (cast `/Game/MyCharacter` _returnvalue))
        (if (`/Game/MyCharacter.HaveObj` _asmy_character_2)
          (set `/Game/MyCharacter.ThinkContent` "I can't take anything with me..." _asmy_character_2)
          (else
            (bind _outactors (`GameplayStatics.GetAllActorsWithTag` "Drop"))
            (for _array_element _outactors
              (`KismetArrayLibrary.Array_Add` (`self.MovableClass`) (`GameplayStatics.GetObjectClass` _array_element))
              (`KismetArrayLibrary.Array_Add` (`self.MovableTransforms`) (`self.GetTransform` _array_element)))
            (set `/Game/MyGameInstance.MovableTransforms` (`self.MovableTransforms`) _asmy_game_instance)
            (set `/Game/MyGameInstance.MovableClasses` (`self.MovableClass`) _asmy_game_instance)
            (set `/Game/MyGameInstance.PlayerTransform` (`self.GetTransform` (`GameplayStatics.GetPlayerCharacter` 0)) _asmy_game_instance)
            (return (`self.LevelName`) true))))
      (return "None" false))))

(fn `TriggerTpHub`
  (returns (Teleport :type Boolean))
  (return false))

(fn `UserConstructionScript`)